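; Health component that tracks an actor's current health and whether it has been defeated.
; Current health starts at the maximum on BeginPlay.
; DecreaseHealth subtracts incoming damage with a floor of zero, prints the result as debug text, and sets IsDefeated once health is depleted.
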(event EventBeginPlay
  (Variables|Default|SetCurrentHealth (Variables|Default|GetMaxHealth)))

(event EventTick
  (params (DeltaSeconds :type Float%20%28single-precision%29)))

(fn DecreaseHealth
  (params (IncomingDamage :type Float%20%28double-precision%29))
  (Variables|Default|SetCurrentHealth (Math|Float|Max(Float) (- (Variables|Default|GetCurrentHealth) IncomingDamage) 0.0))
  (Development|PrintString (Utilities|String|ToString(Float) (Variables|Default|GetCurrentHealth)))
  (Variables|Default|SetIsDefeated (<= (Variables|Default|GetCurrentHealth) 0.0)))